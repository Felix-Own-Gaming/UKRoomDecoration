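; BP_PlaceableObject is a placeable object actor that can switch its look to show a deletion state.
; On BeginPlay it caches the static mesh's first material as the normal material.
; SetMaterial swaps slot 0 between that cached material and a delete material based on an IsDeleting flag, and GetMesh returns the component's static mesh asset.
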(event `self.ReceiveBeginPlay`
  (set `self.NormalMaterial` (`PrimitiveComponent.GetMaterial` (`self.StaticMesh`) 0)))

(fn `GetMesh`
  (returns (Mesh :type "StaticMesh Object Reference"))
  (return (`StaticMeshComponent.StaticMesh` (`self.StaticMesh`))))

(fn `SetMaterial`
  (params (IsDeleting :type Boolean))
  (if IsDeleting
    (`PrimitiveComponent.SetMaterial` (`self.StaticMesh`) 0 (`self.DeleteMaterial`))
    (else
      (`PrimitiveComponent.SetMaterial` (`self.StaticMesh`) 0 (`self.NormalMaterial`)))))

(fn `UserConstructionScript`)