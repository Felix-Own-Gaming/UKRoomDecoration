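; Interactive door object that swings open or closed when its Interact event fires.
; ToogleDoor instantly rotates the Door component 90 degrees in yaw and flips IsOpen, with no animation.
; An XOR of IsForwardOpening and IsOpen picks the rotation sign, so each toggle reverses the previous swing.
; BeginPlay also toggles when IsOpen starts true, which applies the closing rotation and leaves IsOpen false.
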(event `self.ReceiveBeginPlay`
  (`parent.ReceiveBeginPlay`)
  (if (`self.IsOpen`)
    (`self.ToogleDoor`)))

(event `self.ReceiveTick`
  (params (DeltaSeconds :type "Float (single-precision)"))
  (`parent.ReceiveTick` DeltaSeconds))

(event `/Game/BP_Objects/InteractableInterface.Interact`
  ;[1 1 1] OnInteract
  (`self.ToogleDoor`))

(event `ToogleDoor`
  (bind _isopen (`self.IsOpen`))
  (bind _door (`self.Door`))
  (bind _returnvalue (`KismetMathLibrary.Conv_IntToDouble` (`KismetMathLibrary.SelectInt` -90 90 (xor (`self.IsForwardOpening`) _isopen))))
  ;[1 1 1] Toogle Door
  (if _isopen
    (`SceneComponent.K2_AddLocalRotation` _door (`KismetMathLibrary.MakeRotator` 0.0 0.0 _returnvalue) false false)
    (set `self.IsOpen` false)
    (else
      (`SceneComponent.K2_AddLocalRotation` _door (`KismetMathLibrary.MakeRotator` 0.0 0.0 _returnvalue) false false)
      (set `self.IsOpen` true))))

(fn `UserConstructionScript`
  (`parent.UserConstructionScript`))